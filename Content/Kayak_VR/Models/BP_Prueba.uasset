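; BP_Prueba is a test actor that drives itself forward continuously once play begins.
; A Timeline started on BeginPlay applies a fixed local translation and slight rotation on every update, so motion depends on update rate.
; When the Timeline finishes, it prints SpeedB after a zero Delay and restarts from the start.
; The logic that would change SpeedB, including from the Timeline track, is disconnected.
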(event `self.ReceiveBeginPlay`
  (bind (_direction _track_uno) (`Timeline|Timeline_0` :!label _label)
    (:`Update`
      (`self.K2_AddActorLocalTransform` (`KismetMathLibrary.MakeTransform` (100.0 0.0 0.0) (struct :`Yaw` 1.0))))
    (:`Finished`
      (`KismetSystemLibrary.Delay` 0.0)
      (`KismetSystemLibrary.PrintString` (`KismetStringLibrary.Conv_DoubleToString` (`self.Speed_B`)))
      (goto _label :!via `PlayFromStart`))))

(event `self.ReceiveTick`
  (params (DeltaSeconds :type "Float (single-precision)")))

(fn `UserConstructionScript`)