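; Kayak VR actor that travels along the level's BP_Spline path at a speed driven by whether the player is paddling.
; A timeline maps its track to distance along the spline and sets the actor's transform, with play rate derived from TimeToCompleteInSeconds.
; Each update reads Remando from Remo_BP and, through delayed steps, shortens that time toward MaxVelocity while paddling or lengthens it toward MinVelocity otherwise, then reapplies the play rate.
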(event `self.ReceiveBeginPlay`
  (`|ExecutionSequence`
    (:`then_0`
      (bind _returnvalue (`GameplayStatics.GetActorOfClass` "/Game/Kayak_VR/Models/BP_Spline.BP_Spline_C"))
      (set `self.Spline REF` _returnvalue)
      (`self.Move Object`))
    (:`then_1`
      (bind _returnvalue_2 (`GameplayStatics.GetActorOfClass` "/Game/Kayak_VR/Models/Kayak_Model/Remo/Remo_BP.Remo_BP_C"))
      (set `self.remo` _returnvalue_2))))

(event `Move Object`
  (bind _time_to_complete__in_seconds_ (`self.Time To Complete (In Seconds)`))
  (bind _spline (`/Game/Kayak_VR/Models/BP_Spline.Spline` (`self.Spline REF`)))
  (`TimelineComponent.SetPlayRate` (`self.Move Object T`) (/ 1.0 (`self.Time To Complete (In Seconds)`)) :!label _label)
  (bind (_direction _move_track) (`Timeline|Move Object T`)
    (:`Update`
      (`|ExecutionSequence`
        (:`then_0`
          (`KismetSystemLibrary.PrintString` (`KismetStringLibrary.Conv_DoubleToString` _time_to_complete__in_seconds_))
          (bind _returnvalue (`KismetMathLibrary.Lerp` 0.0 (`SplineComponent.GetSplineLength` (`/Game/Kayak_VR/Models/BP_Spline.Spline` (`self.Spline REF`))) _move_track))
          (`self.K2_SetActorTransform` (`KismetMathLibrary.MakeTransform` (`SplineComponent.GetLocationAtDistanceAlongSpline` _spline _returnvalue "World") (`SplineComponent.GetRotationAtDistanceAlongSpline` _spline _returnvalue "Local"))))
        (:`then_1`
          (if (`/Game/Kayak_VR/Models/Kayak_Model/Remo/Remo_BP.remando` (`self.remo`))
            (if (not (<= _time_to_complete__in_seconds_ (`self.maxVelocity`))) :!label _label_2
              (`KismetSystemLibrary.Delay` 0.3)
              (set `self.Time To Complete (In Seconds)` (- _time_to_complete__in_seconds_ 1.0))
              (`|ExecutionSequence`
                (:`then_0`
                  (goto _label_2))
                (:`then_1`
                  (`KismetSystemLibrary.PrintString` "cambio" false :!label _label_3)
                  (goto _label))))
            (else
              (if (not (>= _time_to_complete__in_seconds_ (`self.minVelocity`))) :!label _label_4
                (`KismetSystemLibrary.Delay` 0.3)
                (set `self.Time To Complete (In Seconds)` (+ _time_to_complete__in_seconds_ 1.0))
                (`|ExecutionSequence`
                  (:`then_0`
                    (goto _label_4))
                  (:`then_1`
                    (goto _label_3)))))))))
    (:`Finished`
      (`KismetSystemLibrary.PrintString` "Finalizó el recorrido"))))

(fn `UserConstructionScript`)