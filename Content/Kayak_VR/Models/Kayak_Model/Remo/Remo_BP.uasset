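; Kayak VR paddle actor (Remo) that mirrors the orientation of a physical Arduino controller.
; BeginPlay opens a serial port and polls yaw, pitch and roll on a looping timer to set actor rotation.
; Roll thresholds flag rowing (Remando) and send a vibrate command back.
; MoveObject retunes a timeline's play rate from that flag, but its startup call and spline lookups are disconnected, and Foll's AI follow loop has no outside caller here.
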(event `self.ReceiveBeginPlay`
  (`|ExecutionSequence`
    (:`then_0`
      (bind (_bopened _returnvalue) (`SerialCom.OpenComPort` 4 115200))
      (if _bopened
        (`KismetSystemLibrary.PrintString` "PORT OPEN")
        (set `self.Arduino` _returnvalue)
        (`KismetSystemLibrary.K2_SetTimer` null "readSerialCom" 0.1 true)
        (else
          (`KismetSystemLibrary.PrintString` "PORT NOT OPEN"))))
    (:`then_1`
      (`GameplayStatics.GetActorOfClass` "/Game/VRTemplate/Blueprints/VRPawn.VRPawn_C"))))

(event `self.ReceiveEndPlay`
  (params (EndPlayReason :type "EEndPlayReason Enum" :default "Destroyed"))
  (bind _arduino (`self.Arduino`))
  (`/Engine/EditorBlueprintResources/StandardMacros.IsValid` _arduino
    (:`Is Valid`
      (`SerialCom.Close` _arduino)
      (`KismetSystemLibrary.PrintString` "PORT CLOSED"))
    (:`Is Not Valid`
      (`KismetSystemLibrary.PrintString` "PORT NOT CLOSED"))))

(event `Move Object`
  (bind _timetocomple__in_seconds__ (`self.TimeToComple (in Seconds)}`))
  (bind _remando (`self.remando`))
  (`TimelineComponent.SetPlayRate` (`self.Timeline_0`) (/ 1.0 (`self.TimeToComple (in Seconds)}`)) :!label _label)
  (bind (_direction _move_track) (`Timeline|Timeline_0`)
    (:`Update`
      (`|ExecutionSequence`
        (:`then_0`
          (`KismetSystemLibrary.PrintString` (`KismetStringLibrary.Conv_DoubleToString` _timetocomple__in_seconds__) false))
        (:`then_1`
          (`KismetSystemLibrary.PrintString` (`KismetStringLibrary.Conv_BoolToString` _remando) false)
          (if _remando
            (if (`self.remar`)
              (set `self.remar` false)
              (if (not (<= _timetocomple__in_seconds__ (`self.maxVelocity`))) :!label _label_2
                (`KismetSystemLibrary.Delay` 0.3)
                (set `self.TimeToComple (in Seconds)}` (- _timetocomple__in_seconds__ 20.0))
                (`|ExecutionSequence`
                  (:`then_0`
                    (goto _label_2))
                  (:`then_1`
                    (`KismetSystemLibrary.PrintString` "cambio" false :!label _label_3)
                    (goto _label))))
              (else
                (`KismetSystemLibrary.PrintString` "cambia de lado")))
            (else
              (set `self.remar` true)
              (if (not (>= _timetocomple__in_seconds__ (`self.minVelocity`))) :!label _label_4
                (`KismetSystemLibrary.Delay` 0.3)
                (set `self.TimeToComple (in Seconds)}` (+ _timetocomple__in_seconds__ 5.0))
                (`|ExecutionSequence`
                  (:`then_0`
                    (goto _label_4))
                  (:`then_1`
                    (goto _label_3)))))))))
    (:`Finished`
      (`KismetSystemLibrary.PrintString` "Finalizó el recorrido" false))))

(event `Foll`
  (`|AIMoveTo` (`self.Remo `) null (0.0 0.0 0.0) (`self.vrpawn`)
    (:`then`
      (`KismetSystemLibrary.Delay` 0.2)
      (`KismetSystemLibrary.PrintString` "empiezo")
      (`self.Foll`))))

(fn `readSerialCom`
  (bind (_bsuccess _returnvalue) (`SerialCom.ReadString` (`self.Arduino`)))
  (if (and (> (`KismetStringLibrary.Len` _returnvalue) 13) _bsuccess)
    (bind (_lefts _rights) (`KismetStringLibrary.Split` _returnvalue ","))
    (bind (_lefts_2 _rights_2) (`KismetStringLibrary.Split` _rights ","))
    (bind _returnvalue_2 (`KismetStringLibrary.Conv_StringToDouble` _rights_2))
    (`self.K2_SetActorRotation` (`KismetMathLibrary.MakeRotator` _returnvalue_2 (`KismetStringLibrary.Conv_StringToDouble` _lefts_2) (`KismetStringLibrary.Conv_StringToDouble` _lefts)))
    (`|ExecutionSequence`
      (:`then_0`
        (if (or (>= _returnvalue_2 60.0) (<= _returnvalue_2 -60.0))
          (`SerialCom.Println` (`self.Arduino`) "VIBRATE")))
      (:`then_1`
        (if (or (>= _returnvalue_2 20.0) (<= _returnvalue_2 -20.0))
          (set `self.remando` true)
          (else
            (set `self.remando` false)))))))

(fn `UserConstructionScript`)